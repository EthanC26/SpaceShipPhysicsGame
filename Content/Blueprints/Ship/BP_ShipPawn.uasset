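; Player ship pawn, apparently for a lander game, that manages thruster effects, fuel and health.
; Directional events toggle bottom, left and right thrusters and start a shared sound, which Tick stops once all are off.
; Clamped fuel drives its own WBP_Player widget, while health component changes update HUD_Lander's health bar.
; At zero health, the ship is destroyed and BP_GameMode triggers a losing game over.
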(event Custom|ActivateThrust
  (params (Direction :type Integer))
  ;[0.15 0.15 0.15 0.5] Active Thursters
  (switch int Direction
    (:0
      (if (not (Components|Activation|IsActive (Variables|Default|GetBottomThruster)))
        (Components|Activation|Activate (Variables|Default|GetBottomThruster) false)
        (if (not (Audio|Components|Audio|IsPlaying (Variables|Default|GetAudio))) :!label _label
          (Audio|Components|Audio|Play (Variables|Default|GetAudio) 0.0))))
    (:1
      (if (not (Components|Activation|IsActive (Variables|Default|GetLeftThruster)))
        (Components|Activation|Activate (Variables|Default|GetLeftThruster) false)
        (goto _label)))
    (:2
      (if (not (Components|Activation|IsActive (Variables|Default|GetRightThuster)))
        (Components|Activation|Activate (Variables|Default|GetRightThuster) false)
        (goto _label)))))

(event Custom|DeactivateThrust
  (params (Direction :type Integer))
  ;[0.15 0.15 0.15 0.5] Deactive Thruster
  (switch int Direction
    (:0
      (if (Components|Activation|IsActive (Variables|Default|GetBottomThruster))
        (Components|Activation|Deactivate (Variables|Default|GetBottomThruster))))
    (:1
      (if (Components|Activation|IsActive (Variables|Default|GetLeftThruster))
        (Components|Activation|Deactivate (Variables|Default|GetLeftThruster))))
    (:2
      (if (Components|Activation|IsActive (Variables|Default|GetRightThuster))
        (Components|Activation|Deactivate (Variables|Default|GetRightThuster))))))

(event Custom|ChangeFuel
  (params (ChangeValue :type Float%20%28double-precision%29))
  ;[0.15 0.15 0.15 0.5] Update fuel Bar UI
  (bind _output_get (Variables|Default|SetFuel (Math|Float|Clamp(Float) (+ ChangeValue (Variables|Default|GetFuel)))))
  (Progress|SetPercent (Variables|/Game/Blueprints/GUI/GameMenu/WBP_Player.WBP_Player_C|GetFuelBar (Variables|Default|GetUI)) _output_get))

(event EventBeginPlay
  (bind _returnvalue (Game|ConstructObjectfromClass "/Game/Blueprints/GUI/GameMenu/WBP_Player.WBP_Player_C"))
  (bind _output_get (Variables|Default|SetUI _returnvalue))
  (UserInterface|Viewport|AddtoViewport _output_get 0)
  (CallFunction|ChangeFuel 1.0))

(event Game|Damage|EventAnyDamage
  (params (Damage :type Float%20%28single-precision%29) (DamageType :type Damage%20Type%20Object%20Reference) (InstigatedBy :type Controller%20Object%20Reference) (DamageCauser :type Actor%20Object%20Reference))
  ;[0.15 0.15 0.15 0.5] HandleDamage
  (CallFunction|Damage Damage)
  (if (<= (Default|GetHealth (Variables|Default|GetAC_HealthComponent)) 0.0)
    (Actor|DestroyActor)
    (bind _asbp_game_mode (Utilities|Casting|CastToBP_GameMode (Game|GetGameMode)))
    (Default|GameOverLose _asbp_game_mode)))

(event EventTick
  (params (DeltaSeconds :type Float%20%28single-precision%29))
  (bind _bottomthruster (Variables|Default|GetBottomThruster))
  (bind _leftthruster (Variables|Default|GetLeftThruster))
  (bind _rightthuster (Variables|Default|GetRightThuster))
  (bind _returnvalue (Components|Activation|IsActive _bottomthruster))
  (bind _returnvalue_2 (Components|Activation|IsActive _leftthruster))
  (bind _returnvalue_3 (Components|Activation|IsActive _rightthuster))
  (bind _returnvalue_4 (not _returnvalue_3))
  (bind _returnvalue_5 (not _returnvalue))
  (bind _returnvalue_6 (not _returnvalue_2))
  (bind _returnvalue_7 (Math|Boolean|ANDBoolean _returnvalue_5 _returnvalue_6 _returnvalue_4))
  (if _returnvalue_7
    (if (and (Audio|Components|Audio|IsPlaying (Variables|Default|GetAudio)) _returnvalue_7)
      (Audio|Components|Audio|Stop (Variables|Default|GetAudio)))))

(fn ConstructionScript)

(fn Damage
  (params (DamageAmt :type Float%20%28double-precision%29))
  (Default|Damage (Variables|Default|GetAC_HealthComponent) DamageAmt)
  (CallFunction|UpdateUIHelathBar))

(fn UpdateUIHelathBar
  (bind _ashud_lander (Utilities|Casting|CastToHUD_Lander (HUD|GetHUD (Game|GetPlayerController 0))))
  (Default|SetHealthBar (Variables|/Game/Blueprints/HUD_Lander.HUD_Lander_C|GetMenuRef _ashud_lander) (Default|GetNormalizedHealth (Variables|Default|GetAC_HealthComponent))))

(fn Heal
  (params (HealAmt :type Float%20%28double-precision%29))
  (Default|Heal (Variables|Default|GetAC_HealthComponent) HealAmt)
  (CallFunction|UpdateUIHelathBar))