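; Game mode for a lander game that handles landing and crash outcomes and the level changes that follow.
; BeginPlay hides the cursor and sets game-only input.
; GameOverWin, GameOverLose and NextLevel each write a landed or crashed message to the HUD_Lander menu's bottom text and play a sound.
; After a short delay, they open the win map, game-over map or second game map respectively.
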(event Custom|GameOverWin
  (bind _ashud_lander (Utilities|Casting|CastToHUD_Lander (HUD|GetHUD (Game|GetPlayerController 0))))
  (Rendering|Components|TextRender|SetText (Variables|/Game/Blueprints/GUI/GameMenu/WBP_GameMode.WBP_GameMode_C|GetBottomText (Variables|/Game/Blueprints/HUD_Lander.HUD_Lander_C|GetMenuRef _ashud_lander)) "You have Landed")
  (Audio|PlaySound2D "/Game/Audio/winner-game-sound-404167.winner-game-sound-404167" 1.0 1.0 0.0 0 0)
  (Utilities|FlowControl|Delay 2.0)
  (Game|OpenLevel(byObjectReference) "/Game/Maps/WInMap.WInMap"))

(event Custom|GameOverLose
  (bind _ashud_lander (Utilities|Casting|CastToHUD_Lander (HUD|GetHUD (Game|GetPlayerController 0))))
  (Rendering|Components|TextRender|SetText (Variables|/Game/Blueprints/GUI/GameMenu/WBP_GameMode.WBP_GameMode_C|GetBottomText (Variables|/Game/Blueprints/HUD_Lander.HUD_Lander_C|GetMenuRef _ashud_lander)) "You have Crashed")
  (Audio|PlaySound2D "/Game/Audio/game-over-417465.game-over-417465" 1.0 1.0 0.0 0 0)
  (Utilities|FlowControl|Delay 2.0)
  (Game|OpenLevel(byObjectReference) "/Game/Maps/GameOverMap.GameOverMap"))

(event Custom|NextLevel
  (bind _ashud_lander (Utilities|Casting|CastToHUD_Lander (HUD|GetHUD (Game|GetPlayerController 0))))
  (Rendering|Components|TextRender|SetText (Variables|/Game/Blueprints/GUI/GameMenu/WBP_GameMode.WBP_GameMode_C|GetBottomText (Variables|/Game/Blueprints/HUD_Lander.HUD_Lander_C|GetMenuRef _ashud_lander)) "You have Landed")
  (Audio|PlaySound2D "/Game/Audio/winner-game-sound-404167.winner-game-sound-404167" 1.0 1.0 0.0 0 0)
  (Utilities|FlowControl|Delay 2.0)
  (Game|OpenLevel(byObjectReference) "/Game/Maps/GameMap2.GameMap2"))

(event EventBeginPlay
  (bind _returnvalue (Game|GetPlayerController 0))
  (Variables|/Script/Engine.PlayerController|SetbShowMouseCursor _returnvalue false)
  (Input|SetInputModeGameOnly _returnvalue false))

(fn ConstructionScript)