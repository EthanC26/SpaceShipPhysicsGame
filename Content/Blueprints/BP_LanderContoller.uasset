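; Player controller for a lander game that turns input into thrust on the BP_ShipPawn found in the level at BeginPlay.
; Up and Right axes add physics forces to the ship's RocketMesh while fuel remains, draining fuel over frame time.
; Separate vertical, left and right thruster actions toggle indexed thruster effects on press and release, independently of the fuel check.
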(event EventBeginPlay
  (bind _outactors (Actor|GetAllActorsOfClass "/Game/Blueprints/Ship/BP_ShipPawn.BP_ShipPawn_C"))
  (Variables|Default|SetPlayerShip (Utilities|Array|Get(acopy) _outactors)))

(event Input|ActionEvents|InputActionVerticalThruster
  (params (Key :type Key%20Structure :default "None"))
  ;[0.15 0.15 0.15 0.5] Turn on thruster fx
  (:Pressed
    (Utilities|IsValid (Variables|Default|GetPlayerShip)
      (:Is%20Valid
        (Default|ActivateThrust (Variables|Default|GetPlayerShip)))))
  (:Released
    (Utilities|IsValid (Variables|Default|GetPlayerShip)
      (:Is%20Valid
        (Default|DeactivateThrust (Variables|Default|GetPlayerShip))))))

(event Input|ActionEvents|InputActionLeftThruster
  (params (Key :type Key%20Structure :default "None"))
  ;[0.15 0.15 0.15 0.5] Turn on thruster fx
  (:Pressed
    (Utilities|IsValid (Variables|Default|GetPlayerShip)
      (:Is%20Valid
        (Default|ActivateThrust (Variables|Default|GetPlayerShip) 1))))
  (:Released
    (Utilities|IsValid (Variables|Default|GetPlayerShip)
      (:Is%20Valid
        (Default|DeactivateThrust (Variables|Default|GetPlayerShip) 1)))))

(event Input|ActionEvents|InputActionRightThruster
  (params (Key :type Key%20Structure :default "None"))
  ;[0.15 0.15 0.15 0.5] Turn on thruster fx
  (:Pressed
    (Utilities|IsValid (Variables|Default|GetPlayerShip)
      (:Is%20Valid
        (Default|ActivateThrust (Variables|Default|GetPlayerShip) 2))))
  (:Released
    (Utilities|IsValid (Variables|Default|GetPlayerShip)
      (:Is%20Valid
        (Default|DeactivateThrust (Variables|Default|GetPlayerShip) 2)))))

(event Input|AxisEvents|InputAxisup
  (params (AxisValue :type Float%20%28single-precision%29))
  (bind _playership (Variables|Default|GetPlayerShip))
  ;[0.15 0.15 0.15 0.5] Movement
  (if (> AxisValue 0.01)
    (Utilities|IsValid _playership
      (:Is%20Valid
        (if (> (Variables|/Game/Blueprints/Ship/BP_ShipPawn.BP_ShipPawn_C|GetFuel _playership) 0.0)
          (Physics|AddForce (Variables|/Game/Blueprints/Ship/BP_ShipPawn.BP_ShipPawn_C|GetRocketMesh (Variables|Default|GetPlayerShip)) (Variables|Default|Getforce) "None" false)
          ;[0.15 0.15 0.15 0.5] Change fuel
          (Default|ChangeFuel (Variables|Default|GetPlayerShip) (* (Utilities|Time|GetWorldDeltaSeconds) -0.1)))))))

(event Input|AxisEvents|InputAxisRight
  (params (AxisValue :type Float%20%28single-precision%29))
  (bind _playership (Variables|Default|GetPlayerShip))
  ;[0.15 0.15 0.15 0.5] Movement
  (if (not (Math|Float|NearlyEqual(Float) AxisValue 0.0 0.01))
    (Utilities|IsValid _playership
      (:Is%20Valid
        (if (> (Variables|/Game/Blueprints/Ship/BP_ShipPawn.BP_ShipPawn_C|GetFuel _playership) 0.0)
          (Physics|AddForce (Variables|/Game/Blueprints/Ship/BP_ShipPawn.BP_ShipPawn_C|GetRocketMesh (Variables|Default|GetPlayerShip)) (Math|Vector|MakeVector 0.0 (* AxisValue 1.0) 0.0) "None" false)
          ;[0.15 0.15 0.15 0.5] Change fuel
          (Default|ChangeFuel (Variables|Default|GetPlayerShip) (* (Utilities|Time|GetWorldDeltaSeconds) -0.1)))))))

(fn ConstructionScript)