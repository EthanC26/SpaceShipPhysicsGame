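; BP_Repulser is an obstacle that pushes physics objects away from its location.
; Every tick it sphere-overlaps PhysicsBody actors, excluding itself, and applies a radial impulse of PushStrength to each root primitive component.
; The impulse uses constant falloff and velocity change, ignoring mass; its radius is much smaller than the detection sphere.
; A failed root-component cast ends that tick's processing for that actor.
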(event EventTick
  (params (DeltaSeconds :type Float%20%28single-precision%29))
  (bind _outactors (Collision|SphereOverlapActors (Transformation|GetActorLocation) 7e+02 (Utilities|Array|MakeArray "ObjectTypeQuery4") 0 (Utilities|Array|MakeArray self)))
  (for _array_element _outactors
    (bind _asprimitive_component (Utilities|Casting|CastToPrimitiveComponent (Variables|/Script/Engine.Actor|GetRootComponent _array_element)))
    (Physics|AddRadialImpulse _asprimitive_component (Transformation|GetActorLocation) 2e+02 (Variables|Default|GetPushStrength) "RIF_Constant" true)))

(fn ConstructionScript)