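; BP_BlackHole is an obstacle that applies a radial pull to nearby physics bodies and damages players that hit it.
; Each Tick, it sphere-overlaps for PhysicsBody actors and applies a mass-independent radial impulse of PullStrength to their root primitives.
; The impulse has constant falloff and a much smaller radius than the overlap search.
; Hits on its Sphere component apply DamageAmt to actors implementing BPI_Player.
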(event OnComponentHit(Sphere)
  (params (HitComponent :type Primitive%20Component%20Object%20Reference) (OtherActor :type Actor%20Object%20Reference) (OtherComp :type Primitive%20Component%20Object%20Reference) (NormalImpulse :type Vector :default "0, 0, 0") (Hit :type Hit%20Result%20Structure%20%28by%20ref%29))
  (if (Utilities|DoesObjectImplementInterface OtherActor "/Game/Blueprints/Ship/BPI_Player.BPI_Player_C")
    (Game|Damage|ApplyDamage OtherActor (Variables|Default|GetDamageAmt) 0 0)))

(event EventTick
  (params (DeltaSeconds :type Float%20%28single-precision%29))
  (bind _outactors (Collision|SphereOverlapActors (Transformation|GetActorLocation) 7e+02 (Utilities|Array|MakeArray "ObjectTypeQuery4") 0 (Utilities|Array|MakeArray self)))
  (for _array_element _outactors
    (bind _asprimitive_component (Utilities|Casting|CastToPrimitiveComponent (Variables|/Script/Engine.Actor|GetRootComponent _array_element)))
    (Physics|AddRadialImpulse _asprimitive_component (Transformation|GetActorLocation) 2e+02 (Variables|Default|GetPullStrength) "RIF_Constant" true)))

(fn ConstructionScript)