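; BP_Platform is a landing platform that completes a level for BPI_Player actors and damages those that hit it too hard.
; Unless it is the starting platform, overlap starts a short timer, cancelled on exit, to check whether the player's bounds fit inside the collider along Y.
; A successful check calls BP_GameMode's NextLevel or GameOverWin, depending on IsNextLevelPlatform.
; Platform hits apply damage when player velocity meets a threshold.
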(event OnComponentBeginOverlap(Collider)
  (params (OverlappedComponent :type Primitive%20Component%20Object%20Reference) (OtherActor :type Actor%20Object%20Reference) (OtherComp :type Primitive%20Component%20Object%20Reference) (OtherBodyIndex :type Integer) (bFromSweep :type Boolean) (SweepResult :type Hit%20Result%20Structure%20%28by%20ref%29))
  ;[0.15 0.15 0.15 0.5] First contect with the platform
  (if (and (Utilities|DoesObjectImplementInterface OtherActor "/Game/Blueprints/Ship/BPI_Player.BPI_Player_C") (not (Variables|Default|GetIsStartingPlatform)))
    (Variables|Default|SetOverlappedActor OtherActor)
    (bind _returnvalue (Utilities|Time|SetTimerbyFunctionName 0 "IsPlayerInColliderCheck" 0.1))
    (Variables|Default|SetCollisonCheckTimer _returnvalue)))

(event OnComponentEndOverlap(Collider)
  (params (OverlappedComponent :type Primitive%20Component%20Object%20Reference) (OtherActor :type Actor%20Object%20Reference) (OtherComp :type Primitive%20Component%20Object%20Reference) (OtherBodyIndex :type Integer))
  ;[0.15 0.15 0.15 0.5] End contact with the platform
  (if (and (Utilities|DoesObjectImplementInterface OtherActor "/Game/Blueprints/Ship/BPI_Player.BPI_Player_C") (not (Variables|Default|GetIsStartingPlatform)))
    (Utilities|Time|ClearandInvalidateTimerbyHandle (Variables|Default|GetCollisonCheckTimer))))

(event OnComponentHit(Platform)
  (params (HitComponent :type Primitive%20Component%20Object%20Reference) (OtherActor :type Actor%20Object%20Reference) (OtherComp :type Primitive%20Component%20Object%20Reference) (NormalImpulse :type Vector :default "0, 0, 0") (Hit :type Hit%20Result%20Structure%20%28by%20ref%29))
  ;[0.15 0.15 0.15 0.5] Check if hit platform to hard & if yes damage player
  (if (and (Utilities|DoesObjectImplementInterface OtherActor "/Game/Blueprints/Ship/BPI_Player.BPI_Player_C") (>= (Math|Vector|VectorLength (Transformation|GetVelocity OtherActor)) 5e+01))
    (Game|Damage|ApplyDamage OtherActor (Variables|Default|GetDamageAmt) 0 0)))

(event Custom|IsPlayerInColliderCheck
  (bind _collider (Variables|Default|GetCollider))
  (bind _overlappedactor (Variables|Default|GetOverlappedActor))
  (bind (_origin _boxextent) (Collision|GetComponentBounds _collider))
  (bind (_origin_2 _boxextent_2) (Collision|GetActorBounds _overlappedactor true false))
  ;[0.15 0.15 0.15 0.5] Collision
  (if (<= (Math|Float|Absolute(Float) (- (.y _origin) (.y _origin_2))) (- (.y _boxextent) (.y _boxextent_2)))
    (if (not (Variables|Default|GetIsNextLevelPlatform))
      (Utilities|Time|ClearandInvalidateTimerbyHandle (Variables|Default|GetCollisonCheckTimer))
      (bind _asbp_game_mode (Utilities|Casting|CastToBP_GameMode (Game|GetGameMode)))
      (Default|GameOverWin _asbp_game_mode)
      (else
        (Utilities|Time|ClearandInvalidateTimerbyHandle (Variables|Default|GetCollisonCheckTimer))
        (bind _asbp_game_mode_2 (Utilities|Casting|CastToBP_GameMode (Game|GetGameMode)))
        (Default|NextLevel _asbp_game_mode_2)))))

(fn ConstructionScript)